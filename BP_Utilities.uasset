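; BP_Utilities is a set of helper functions for color conversion, star positioning and a post-process fade.
; Color helpers parse hex strings into normalized RGB, turn B-V color index into Kelvin, and approximate Kelvin as RGB with piecewise log/power curves.
; RADECToCartesian converts right ascension, declination and parsecs into XYZ coordinates in light-years.
; FilmicFade overwrites the first PostProcessVolume's settings using a given amount.
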(fn `B-V_to_Kelvin`
  (params (ColorIndex :type "Float (double-precision)"))
  (returns (Kelvin :type "Float (double-precision)"))
  (return (* (+ (/ 1.0 (+ (* 0.92 ColorIndex) 0.62)) (/ 1.0 (+ (* 0.92 ColorIndex) 1.7))) 4700.0)))

(fn `CalculateHex`
  (params (Hex :type String))
  (returns (Decimal :type "Float (double-precision)"))
  (if (`KismetStringLibrary.IsNumeric` Hex)
    (return (`KismetStringLibrary.Conv_StringToDouble` Hex))
    (else
      (switch `string` Hex
        (:`A`
          (return 10.0))
        (:`B`
          (return 11.0))
        (:`C`
          (return 12.0))
        (:`D`
          (return 13.0))
        (:`E`
          (return 14.0))
        (:`F`
          (return 15.0))))))

(fn `FilmicFade`
  (params (amount :type "Float (double-precision)"))
  (bind _outactors (`GameplayStatics.GetAllActorsOfClass` null "/Script/Engine.PostProcessVolume"))
  (set `PostProcessVolume.Settings` (make `PostProcessSettings` :`AutoExposureBias` amount) (`|GetArrayItem` _outactors)))

(fn `HexToRGB`
  (params (Hex :type String))
  (returns (Color :type "LinearColor Structure"))
  (locals (R :type "Float (double-precision)") (B :type "Float (double-precision)") (G :type "Float (double-precision)"))
  (bind (_lefts _rights _returnvalue) (`KismetStringLibrary.Split` Hex "#"))
  (bind _returnvalue_2 (select `bool` _returnvalue :`false` Hex :`true` _rights))
  (bind _returnvalue_3 (`KismetStringLibrary.GetSubstring` _returnvalue_2 4 2))
  (bind _returnvalue_4 (`KismetStringLibrary.GetSubstring` _returnvalue_2 0 2))
  (bind _returnvalue_5 (`KismetStringLibrary.GetSubstring` _returnvalue_2 2 2))
  ;[1 1 1] R
  (bind _decimal (`self.CalculateHex` (`KismetStringLibrary.GetSubstring` _returnvalue_4)))
  (bind _decimal_2 (`self.CalculateHex` (`KismetStringLibrary.GetSubstring` _returnvalue_4 1)))
  (set `local.R` (+ (* _decimal (`KismetMathLibrary.MultiplyMultiply_FloatFloat` 16.0 1.0)) (* _decimal_2 (`KismetMathLibrary.MultiplyMultiply_FloatFloat` 16.0 0.0))))
  ;[1 1 1] G
  (bind _decimal_3 (`self.CalculateHex` (`KismetStringLibrary.GetSubstring` _returnvalue_5)))
  (bind _decimal_4 (`self.CalculateHex` (`KismetStringLibrary.GetSubstring` _returnvalue_5 1)))
  (set `local.G` (+ (* _decimal_3 (`KismetMathLibrary.MultiplyMultiply_FloatFloat` 16.0 1.0)) (* _decimal_4 (`KismetMathLibrary.MultiplyMultiply_FloatFloat` 16.0))))
  ;[1 1 1] B
  (bind _decimal_5 (`self.CalculateHex` (`KismetStringLibrary.GetSubstring` _returnvalue_3)))
  (bind _decimal_6 (`self.CalculateHex` (`KismetStringLibrary.GetSubstring` _returnvalue_3 1)))
  (set `local.B` (+ (* _decimal_5 (`KismetMathLibrary.MultiplyMultiply_FloatFloat` 16.0 1.0)) (* _decimal_6 (`KismetMathLibrary.MultiplyMultiply_FloatFloat` 16.0))))
  (return (make `LinearColor` (/ (`local.R`) 255.0) (/ (`local.G`) 255.0) (/ (`local.B`) 255.0) 1.0)))

(fn `KelvinToRGB`
  (params (Kelvin :type "Float (double-precision)"))
  (returns (NewParam :type "LinearColor Structure"))
  (locals (Temperature :type "Float (double-precision)") (Red :type "Float (double-precision)") (Green :type "Float (double-precision)") (Blue :type "Float (double-precision)"))
  (set `local.Temperature` (/ Kelvin 100.0))
  ;[1 0 0] Calculate red
  (if (<= (`local.Temperature`) 66.0)
    (set `local.Red` 255.0)
    (else
      (set `local.Red` (* 329.69873 (`KismetMathLibrary.MultiplyMultiply_FloatFloat` (- (`local.Temperature`) 60.0) -0.133205)))
      (if (< (`local.Red`) 0.0)
        (set `local.Red` 0.0)
        (elif (> (`local.Red`) 255.0)
          (set `local.Red` 255.0)))))
  ;[0 1 0] Calculate green
  (if (<= (`local.Temperature`) 66.0)
    (set `local.Green` (- (* 99.470802 (`KismetMathLibrary.Loge` (`local.Temperature`))) 161.119568))
    (if (< (`local.Green`) 0.0)
      (set `local.Green` 0.0)
      (elif (> (`local.Green`) 255.0)
        (set `local.Green` 255.0)
        (else
          (set `local.Green` (* 288.122162 (`KismetMathLibrary.MultiplyMultiply_FloatFloat` (- (`local.Temperature`) 60.0) -0.075515)) :!label _label)
          (if (< (`local.Green`) 0.0)
            (set `local.Green` 0.0)
            (elif (> (`local.Green`) 255.0)
              (set `local.Green` 255.0))))))
    (else
      (goto _label)))
  ;[0 0 1] Calculate blue
  (if (>= (`local.Temperature`) 66.0)
    (set `local.Blue` 255.0)
    (elif (<= (`local.Temperature`) 19.0)
      (set `local.Blue` 0.0)
      (else
        (set `local.Blue` (- (* 138.517731 (`KismetMathLibrary.Loge` (- (`local.Temperature`) 10.0))) 305.0448))
        (if (< (`local.Blue`) 0.0)
          (set `local.Blue` 0.0)
          (elif (> (`local.Blue`) 255.0)
            (set `local.Blue` 255.0))))))
  (return (make `LinearColor` (/ (`local.Red`) 255.0) (/ (`local.Green`) 255.0) (/ (`local.Blue`) 255.0) 1.0)))

(fn `RADEC_to_Cartesian`
  (params (RA_Hours :type "Float (double-precision)") (RA_Minutes :type "Float (double-precision)") (RA_Seconds :type "Float (double-precision)") (DEC_Degrees :type "Float (double-precision)") (DEC_Minutes :type "Float (double-precision)") (DEC_Seconds :type "Float (double-precision)") (Parsecs :type "Float (double-precision)"))
  (returns (Location :type "Vector Structure"))
  (bind _returnvalue (* Parsecs 3.262))
  (bind _returnvalue_2 (+ (* RA_Hours 15.0) (* RA_Minutes 0.25) (* RA_Seconds 0.004166)))
  (bind _returnvalue_3 (* (+ (`KismetMathLibrary.Abs` DEC_Degrees) (/ DEC_Minutes 60.0) (/ DEC_Seconds 3600.0)) (`KismetMathLibrary.SignOfFloat` DEC_Degrees)))
  (bind _returnvalue_4 (* (`KismetMathLibrary.DegCos` _returnvalue_3) _returnvalue))
  (return (`KismetMathLibrary.MakeVector` (* _returnvalue_4 (`KismetMathLibrary.DegSin` _returnvalue_2)) (* _returnvalue_4 (`KismetMathLibrary.DegCos` _returnvalue_2)) (* (`KismetMathLibrary.DegSin` _returnvalue_3) _returnvalue))))